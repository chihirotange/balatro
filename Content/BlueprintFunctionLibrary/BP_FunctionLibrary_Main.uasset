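; Blueprint function library that gives any Blueprint static helpers to emit card game events for a Balatro-style game.
; Play, discard and deal helpers, covering both commands and per-card events, forward to broadcast functions on the event manager.
; GetMainEventManager casts the GameState to BalatroGameState, which acts as that manager, and prints an error if the cast fails.
; UnsubscribeAllListeners clears all listeners through the same manager.
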(fn `EmitDealCardEvent`
  (params (Card :type "Card Object Reference"))
  (`BalatroGameState.BroadcastDealCard` (`self.GetMainEventManager` null) Card))

(fn `EmitDealCardsCommand`
  (`BalatroGameState.BroadcastDealCardCommand` (`self.GetMainEventManager` null)))

(fn `EmitDiscardCardEvent`
  (params (Card :type "Card Object Reference") (IsLastCard :type Boolean))
  (`BalatroGameState.BroadcastDiscardCard` (`self.GetMainEventManager` null) Card IsLastCard))

(fn `EmitDiscardCommand`
  (`BalatroGameState.BroadcastDiscardCommand` (`self.GetMainEventManager` null)))

(fn `EmitPlayCardEvent`
  (params (Card :type "Card Object Reference") (IsLastCard :type Boolean))
  (`BalatroGameState.BroadcastPlayCardAction` (`self.GetMainEventManager` null) Card IsLastCard))

(fn `EmitPlayCommand`
  (`BalatroGameState.BroadcastPlayCommand` (`self.GetMainEventManager` null)))

(fn `GetMainEventManager`
  (returns (`AsBalatro Game State` :type "BalatroGameState Object Reference"))
  (bind _asbalatro_game_state (cast `BalatroGameState` (`GameplayStatics.GetGameState` null))
    (:`then`
      (return _asbalatro_game_state))
    (:`CastFailed`
      (`KismetSystemLibrary.PrintString` null "COUDLN'T CAST TO BALATRO GAME STATE!!!" true true (struct :`R` 1.0 :`B` 0.096547 :`A` 1.0)))))

(fn `UnsubscribeAllListeners`
  (`BalatroGameState.UnsubscribeAllListeners` (`self.GetMainEventManager` null)))