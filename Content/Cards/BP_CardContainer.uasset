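; Card hand container that lays out cards across a zone, using a vector curve for X spread, height and rotation.
; Dealt, played and discarded events update the card list and recompute each card's origin.
; While a card is grabbed, Tick compares its X to other cards' origins and swaps those it passes, enabling drag reordering.
; The construction script previews evenly spaced slots with instances; SpawnCards is a disconnected stub.
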(event `self.ReceiveBeginPlay`
  (`parent.ReceiveBeginPlay`)
  (`self.SpawnCards`)
  (`self.ModifyCardPositionBasedOnCurve`))

(event `self.ReceiveTick`
  (params (DeltaSeconds :type "Float (single-precision)"))
  (`parent.ReceiveTick` DeltaSeconds)
  (`self.CheckIfShouldSwapCard`))

(event `/Game/Interfaces/I_GrabEventListener.OnTargetGrabbed`
  (params (GrabbedActor :type "Actor Object Reference"))
  (set `self.GrabbedCard` GrabbedActor)
  (`self.SetActorTickEnabled` true))

(event `/Game/Interfaces/I_GrabEventListener.OnTargetReleased`
  ;[1 1 1] dangerous (what if something interupt this and tick cannot enable?)
  (`self.SetActorTickEnabled` false))

(event `self.GameplayEventListener.OnCardDealt`
  (params (Card :type "Card Object Reference"))
  (`|ExecutionSequence`
    (:`then_0`
      (message `/Game/Interfaces/I_Grabbable.AddGrabEventListener` Card self)
      (`KismetArrayLibrary.Array_AddUnique` (`self.CardsList`) Card)
      (`/Engine/EditorBlueprintResources/StandardMacros.IncrementInt` (`self.NumberOfCards`)))
    (:`then_1`
      (`self.RepositionCards`))))

(event `self.GameplayEventListener.OnCardPlayed`
  (params (Card :type "Card Object Reference"))
  (`KismetArrayLibrary.Array_RemoveItem` (`self.CardsList`) Card)
  (`self.RepositionCards`))

(event `self.GameplayEventListener.OnCardDiscarded`
  (params (Card :type "Card Object Reference"))
  (`KismetArrayLibrary.Array_RemoveItem` (`self.CardsList`) Card)
  (`self.RepositionCards`))

(fn `CalculateIndividualCardTransform`
  (params (CardIndex :type Integer) (MaxRotation :type "Float (double-precision)") (MaxYOffset :type "Float (double-precision)"))
  (returns (NewParam :type "Vector Structure") (Rotation :type "Float (double-precision)"))
  (bind (_returnvalue_x _returnvalue_y _returnvalue_z) (`KismetMathLibrary.BreakVector` (`self.K2_GetActorLocation`)))
  (bind _zonesize_x (`KismetMathLibrary.BreakVector2D` (`self.ZoneSize`)))
  (bind (_returnvalue_x_2 _returnvalue_y_2 _returnvalue_z_2) (`KismetMathLibrary.BreakVector` (`CurveVector.GetVectorValue` (`self.TransformCurve`) (/ (`KismetMathLibrary.Conv_IntToDouble` CardIndex) (`KismetMathLibrary.Conv_IntToDouble` (- (`self.NumberOfCards`) 1))))))
  (return (`KismetMathLibrary.MakeVector` (+ (* _returnvalue_x_2 _zonesize_x) _returnvalue_x) (+ (`KismetMathLibrary.Conv_IntToDouble` CardIndex) _returnvalue_y) (+ _returnvalue_z (* _returnvalue_y_2 MaxYOffset))) (* _returnvalue_z_2 MaxRotation)))

(fn `CheckIfShouldSwapCard`
  (locals (CachedOrigin :type "Vector Structure" :default (0.0 0.0 0.0)))
  (bind _returnvalue_x (`KismetMathLibrary.BreakVector` (`self.K2_GetActorLocation` (`self.GrabbedCard`))))
  (for _array_element (`self.CardsList`)
    (bind _origin (message `/Game/Interfaces/I_HasPositionOrigin.GetOrigin` _array_element))
    (if (> _returnvalue_x (.x _origin))
      (bind _origin_2 (message `/Game/Interfaces/I_HasPositionOrigin.GetOrigin` (`self.GrabbedCard`)))
      (if (> (.x _origin) (.x _origin_2))
        (message `/Game/Interfaces/I_Movable.SwapWithOther` _array_element (`self.GrabbedCard`) :!label _label))
      (else
        (bind _origin_3 (message `/Game/Interfaces/I_HasPositionOrigin.GetOrigin` (`self.GrabbedCard`)))
        (if (< (.x _origin) (.x _origin_3))
          (goto _label))))))

(fn `ModifyCardPositionBasedOnCurve`
  (for (_array_element _array_index) (`self.CardsList`)
    (bind (_newparam _rotation) (`self.CalculateIndividualCardTransform` _array_index -10.0 10.0))
    (message `/Game/Interfaces/I_HasPositionOrigin.SetOrigin` _array_element _newparam)
    (message `/Game/Interfaces/I_HasPositionOrigin.SetOriginRotation` _array_element _rotation)))

(fn `RepositionCards`
  (set `self.NumberOfCards` (`KismetArrayLibrary.Array_Length` (`self.CardsList`)))
  (for (_array_element _array_index) (`self.CardsList`)
    (bind (_newparam _rotation) (`self.CalculateIndividualCardTransform` _array_index -10.0 10.0))
    (message `/Game/Interfaces/I_HasPositionOrigin.SetOrigin` _array_element _newparam)
    (message `/Game/Interfaces/I_HasPositionOrigin.SetOriginRotation` _array_element _rotation)))

(fn `SpawnCards`
  (locals (Origin :type "Vector Structure")))

(fn `UserConstructionScript`
  (bind _zonesize_x (`KismetMathLibrary.BreakVector2D` (`self.ZoneSize`)))
  (bind _zonesize_x_2 (`KismetMathLibrary.BreakVector2D` (`self.ZoneSize`)))
  (bind (_returnvalue_x _returnvalue_y) (`KismetMathLibrary.BreakVector2D` (/ (`self.ZoneSize`) (2.0 2.0))))
  (`InstancedStaticMeshComponent.ClearInstances` (`self.LocationVisualization`))
  (`BoxComponent.SetBoxExtent` (`self.ZoneVisualization`) (`KismetMathLibrary.MakeVector` _returnvalue_x 0.0 _returnvalue_y) true)
  (for _index (range (`self.NumberOfCards`))
    (`InstancedStaticMeshComponent.AddInstance` (`self.LocationVisualization`) (`KismetMathLibrary.MakeTransform` (`KismetMathLibrary.MakeVector` (- (* _index (/ _zonesize_x (- (`self.NumberOfCards`) 1))) (/ _zonesize_x_2 2.0)))) false)))