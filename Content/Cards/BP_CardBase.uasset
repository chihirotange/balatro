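; Base card actor with a widget face and box collider that can be hovered, selected, grabbed, swapped and disposed of.
; Tick lerps it toward TargetLocation while grabbed, otherwise toward Origin, tilting it by remaining X distance.
; Grab and release notify registered listeners, and Swap exchanges origin and rotation with another card.
; Hover rolls the widget via timeline, selection offsets it, and data asset changes refresh its displayed value.
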(event `TempActorTIckEnable`
  (params (Duration :type "Float (single-precision)"))
  (`self.SetActorTickEnabled` true)
  (`KismetSystemLibrary.Delay` Duration)
  (`self.SetActorTickEnabled` false))

(event `self.ReceiveBeginPlay`
  (`parent.ReceiveBeginPlay`)
  (`|ExecutionSequence`
    (:`then_0`
      (bind _output_get (set `self.Origin` (`self.K2_GetActorLocation`)))
      (set `self.TargetLocation` _output_get))
    (:`then_1`
      (`self.SetTimelinePlayrates`))))

(event `self.ReceiveTick`
  (params (DeltaSeconds :type "Float (single-precision)"))
  (`parent.ReceiveTick` DeltaSeconds)
  (if (`self.IsGrabbed`)
    (`self.SetLocationWhenBeingGrabbed`)
    (else
      (`self.SetLocationWhenNotGrabbed`))))

(event `/Game/Interfaces/I_Grabbable.AddGrabEventListener`
  (params (Listener :type "/Game/Interfaces/I_GrabEventListener Interface"))
  (`KismetArrayLibrary.Array_AddUnique` (`self.GrabEventListeners`) Listener))

(event `/Game/Interfaces/I_CardState.OnSelected`
  (`SceneComponent.K2_SetRelativeLocation` (`self.Widget`) (0.0 0.0 50.0) false false))

(event `/Game/Interfaces/I_Grabbable.OnGrabbed`
  (`|ExecutionSequence`
    (:`then_0`
      (for _array_element (`self.GrabEventListeners`)
        (`/Game/Interfaces/I_GrabEventListener.OnTargetGrabbed` _array_element self)
        (set `self.IsGrabbed` true)))
    (:`then_1`
      (`self.SetActorTickEnabled` true))))

(event `/Game/Interfaces/I_CardState.OnDeselected`
  (`SceneComponent.ResetRelativeTransform` (`self.Widget`)))

(event `/Game/Interfaces/I_Grabbable.OnRelease`
  (bind (_returnvalue_x _returnvalue_y _returnvalue_z) (`KismetMathLibrary.BreakVector` (`self.K2_GetActorLocation`)))
  (bind (_origin_x _origin_y) (`KismetMathLibrary.BreakVector` (`self.Origin`)))
  (for _array_element (`self.GrabEventListeners`)
    (`/Game/Interfaces/I_GrabEventListener.OnTargetReleased` _array_element)
    (set `self.IsGrabbed` false)
    ;[1 1 1] So this card won't obstruct other cards when going back to origin
    (`self.K2_SetActorLocation` (`KismetMathLibrary.MakeVector` _returnvalue_x _origin_y _returnvalue_z))))

(event `/Game/Interfaces/I_HasPositionOrigin.SetOrigin`
  (params (NewOrigin :type "Vector Structure"))
  (set `self.Origin` NewOrigin))

(event `/Game/Interfaces/I_Movable.SetNewLocation`
  (params (Location :type "Vector Structure"))
  (set `self.TargetLocation` Location))

(event `/Game/Interfaces/I_HasPositionOrigin.SetOriginRotation`
  (params (Rotation :type "Float (double-precision)"))
  (set `self.OriginRotation` Rotation))

(event `/Game/Interfaces/I_Movable.SwapWithOther`
  (params (SwapWith :type "Actor Object Reference"))
  (`self.Swap` SwapWith))

(event `/Game/Interfaces/I_Grabbable.OnHovered`
  (bind (_direction _newtrack_0) (`Timeline|OhHovered` :!via `PlayFromStart`)
    (:`Update`
      (`SceneComponent.K2_SetRelativeRotation` (`self.Widget`) (`KismetMathLibrary.MakeRotator` (* _newtrack_0 10.0)) false false))))

(event `self.DataAssetContainer.OnDataAssetChanged`
  ;[1 1 1] @TODO: this is dirty and a temp, trying to make it cleaner
  (bind _returnvalue (`HasValue.GetValue`))
  (message `HasValue.SetValue` (`WidgetComponent.GetUserWidgetObject` (`self.Widget`)) _returnvalue))

(event `self.Dispose`
  ;[1 1 1] @TODO: Temp
  (`KismetSystemLibrary.DelayUntilNextTick` :!label _label)
  (`self.K2_DestroyActor`))

(event `self.Use`
  ;[1 1 1] @TODO: Temp
  (goto _label))

(fn `GetOrigin`
  (returns (Origin :type "Vector Structure"))
  (return (`self.Origin`)))

(fn `GetOriginRotation`
  (returns (Rotation :type "Float (double-precision)"))
  (return (`self.OriginRotation`)))

(fn `SetCardName`
  (params (Name :type String))
  (message `/Game/Interfaces/UI/I_SetName.SetName` (`WidgetComponent.GetWidget` (`self.Widget`)) Name))

(fn `SetLocationWhenBeingGrabbed`
  (bind _returnvalue_x (`KismetMathLibrary.BreakVector` (* (`KismetMathLibrary.ClampVectorSize` (- (`self.TargetLocation`) (`self.K2_GetActorLocation`)) 0.0 1000.0) (0.2 0.0 0.0))))
  (`self.K2_SetActorLocation` (`KismetMathLibrary.VLerp` (`self.K2_GetActorLocation`) (`self.TargetLocation`) 0.1))
  (`self.K2_SetActorRotation` (`KismetMathLibrary.MakeRotator` 0.0 _returnvalue_x)))

(fn `SetLocationWhenNotGrabbed`
  (bind _returnvalue_x (`KismetMathLibrary.BreakVector` (* (`KismetMathLibrary.ClampVectorSize` (- (`self.Origin`) (`self.K2_GetActorLocation`)) 0.0 1000.0) (0.2 0.0 0.0))))
  (`|ExecutionSequence`
    (:`then_0`
      (`self.K2_SetActorLocation` (`KismetMathLibrary.VLerp` (`self.K2_GetActorLocation`) (`self.Origin`) 0.09)))
    (:`then_1`
      (`self.K2_SetActorRotation` (`KismetMathLibrary.MakeRotator` 0.0 (+ _returnvalue_x (`self.OriginRotation`)))))))

(fn `SetTimelinePlayrates`
  (`TimelineComponent.SetPlayRate` (`self.OhHovered`) 3.0))

(fn `Swap`
  (params (Actor :type "Actor Object Reference"))
  (locals (TempLoc :type "Vector Structure" :default (0.0 0.0 0.0)) (TempRot :type "Float (double-precision)" :default 0.0))
  (`|ExecutionSequence`
    (:`then_0`
      (bind _origin (message `/Game/Interfaces/I_HasPositionOrigin.GetOrigin` Actor))
      (set `local.TempLoc` _origin))
    (:`then_1`
      (bind _rotation (message `/Game/Interfaces/I_HasPositionOrigin.GetOriginRotation` Actor))
      (set `local.TempRot` _rotation))
    (:`then_2`
      (message `/Game/Interfaces/I_HasPositionOrigin.SetOrigin` Actor (`self.Origin`))
      (message `/Game/Interfaces/I_HasPositionOrigin.SetOriginRotation` Actor (`self.OriginRotation`)))
    (:`then_3`
      (set `self.Origin` (`local.TempLoc`))
      (set `self.OriginRotation` (`local.TempRot`)))))

(fn `UserConstructionScript`
  (bind (_returnvalue_x _returnvalue_y) (`KismetMathLibrary.BreakVector2D` (/ (`self.CardSize`) (2.0 2.0))))
  (`WidgetComponent.SetDrawSize` (`self.Widget`) (`self.CardSize`))
  (`BoxComponent.SetBoxExtent` (`self.Collider`) (`KismetMathLibrary.MakeVector` 20.0 _returnvalue_x _returnvalue_y) false))