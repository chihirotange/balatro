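; Game state for a Balatro-style card game that keeps the score as cards are played.
; Listens for the OnCardPlayed gameplay event and adds each card's value, fetched by a GetValue message call, to a running calculated score.
; On the last card it banks that running score into the current score and resets it, printing both totals to screen.
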(event `self.GameplayEventListener.OnCardPlayed`
  (params (Card :type "Card Object Reference") (IsLastCard :type Boolean))
  (bind _returnvalue (message `HasValue.GetValue` Card))
  (set `self.CurrentCalculatedScore` (+ (`self.CurrentCalculatedScore`) _returnvalue))
  (`KismetSystemLibrary.PrintString` (`KismetStringLibrary.Conv_Int64ToString` (`self.CurrentCalculatedScore`)) true true (struct :`R` 1.0 :`G` 0.087406 :`A` 1.0))
  (if IsLastCard
    (set `self.CurrentScore` (+ (`self.CurrentScore`) (`self.CurrentCalculatedScore`)))
    (set `self.CurrentCalculatedScore` 0)
    (`KismetSystemLibrary.PrintString` (`KismetStringLibrary.Conv_Int64ToString` (`self.CurrentScore`)))))

(fn `UserConstructionScript`)