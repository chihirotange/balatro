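; Player controller for a Balatro-style card game that handles mouse hovering and dragging of cards.
; On BeginPlay it finds or spawns the main camera, shows the cursor and adds the input mapping.
; Drag input sphere-traces along Y at the deprojected cursor, then moves I_Grabbable actors each Tick with a stored XZ offset until release.
; When not dragging, Tick line-traces likewise, caching the hit I_CardState actor to avoid repeated hover messages.
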(event `self.ReceiveBeginPlay`
  (`parent.ReceiveBeginPlay`)
  (`|ExecutionSequence`
    (:`then_0`
      (`self.SetupCamera`)
      (set `self.bShowMouseCursor` true)
      (set `self.bEnableMouseOverEvents` true))
    (:`then_1`
      (`EnhancedInputSubsystemInterface.AddMappingContext` (subsystem `EnhancedInputLocalPlayerSubsystem`) "/Game/Input/IMC_Default.IMC_Default" 0 (struct)))))

(event `EnhancedInput|/Game/Input/IA_Drag`
  (params (ActionValue :type Boolean) (ElapsedSeconds :type "Float (double-precision)") (TriggeredSeconds :type "Float (double-precision)") (InputAction :type "InputAction Object Reference" :default "/Game/Input/IA_Drag.IA_Drag"))
  (bind _worldlocation (`self.DeprojectMousePositionToWorld`))
  (:`Started`
    (bind _outhit (`KismetSystemLibrary.SphereTraceSingleForObjects` (`KismetMathLibrary.MakeVector` (.x _worldlocation) 900.0 (.z _worldlocation)) (`KismetMathLibrary.MakeVector` (.x _worldlocation) -900.0 (.z _worldlocation)) 1.0 (`|MakeArray` "ObjectTypeQuery2" :!type "EObjectTypeQuery Enum")))
    (if (`KismetSystemLibrary.DoesImplementInterface` (`.HitActor` (`GameplayStatics.BreakHitResult` _outhit)) "/Game/Interfaces/I_Grabbable.I_Grabbable_C")
      (set `self.IsDragging` true)
      (bind _output_get (set `self.CurrentlySnappedActorsUnderCursor` (`.HitActor` (`GameplayStatics.BreakHitResult` _outhit))))
      (message `/Game/Interfaces/I_Grabbable.OnGrabbed` _output_get)
      (message `/Game/Interfaces/I_CardState.OnDeselected` (`self.CurrentlySnappedActorsUnderCursor`))
      (bind (_returnvalue_x _returnvalue_y _returnvalue_z) (`KismetMathLibrary.BreakVector` (- (`self.K2_GetActorLocation` _output_get) (`self.DeprojectMousePositionToWorld`))))
      (set `self.DragOffset` (`KismetMathLibrary.MakeVector` _returnvalue_x 0.0 _returnvalue_z))))
  (:`Canceled`
    (set `self.IsDragging` false :!label _label)
    (message `/Game/Interfaces/I_Grabbable.OnRelease` (`self.CurrentlySnappedActorsUnderCursor`))
    (`self.ResetDragParams`))
  (:`Completed`
    (goto _label)))

(event `EnhancedInput|/Game/Input/IA_Click`
  (params (ActionValue :type Boolean) (ElapsedSeconds :type "Float (double-precision)") (TriggeredSeconds :type "Float (double-precision)") (InputAction :type "InputAction Object Reference" :default "/Game/Input/IA_Click.IA_Click")))

(event `self.ReceiveTick`
  (params (DeltaSeconds :type "Float (single-precision)"))
  (bind _worldlocation (`self.DeprojectMousePositionToWorld`))
  (`parent.ReceiveTick` DeltaSeconds)
  (if (`self.IsDragging`)
    (message `/Game/Interfaces/I_Movable.SetNewLocation` (`self.CurrentlySnappedActorsUnderCursor`) (+ (`self.DragOffset`) (`self.DeprojectMousePositionToWorld`)))
    (else
      (bind (_outhit _returnvalue) (`KismetSystemLibrary.LineTraceSingleForObjects` (`KismetMathLibrary.MakeVector` (.x _worldlocation) 900.0 (.z _worldlocation)) (`KismetMathLibrary.MakeVector` (.x _worldlocation) -900.0 (.z _worldlocation)) (`|MakeArray` "ObjectTypeQuery2" :!type "EObjectTypeQuery Enum")))
      (if _returnvalue
        (if (and (`KismetSystemLibrary.DoesImplementInterface` (`.HitActor` (`GameplayStatics.BreakHitResult` _outhit)) "/Game/Interfaces/I_CardState.I_CardState_C") (!= (`self.ActorUnderCursor`) (`.HitActor` (`GameplayStatics.BreakHitResult` _outhit))))
          (message `/Game/Interfaces/I_Grabbable.OnHovered` (`.HitActor` (`GameplayStatics.BreakHitResult` _outhit)))
          (set `self.ActorUnderCursor` (`.HitActor` (`GameplayStatics.BreakHitResult` _outhit))))
        (else
          (set `self.ActorUnderCursor` null))))))

(fn `CalculateCurrentGrabbedActorVelocity`
  (returns (X :type "Float (double-precision)"))
  (bind _returnvalue_x (`KismetMathLibrary.BreakVector` (* (`KismetMathLibrary.ClampVectorSize` (- (`self.DeprojectMousePositionToWorld`) (`self.K2_GetActorLocation` (`self.CurrentlySnappedActorsUnderCursor`))) 0.0 1000.0) (0.2 0.0 0.0))))
  (return _returnvalue_x))

(fn `ResetDragParams`
  (set `self.CurrentlySnappedActorsUnderCursor` null)
  (set `self.DragOffset` (0.0 0.0 0.0)))

(fn `SetupCamera`
  (`|ExecutionSequence`
    (:`then_0`
      (bind _returnvalue (`GameplayStatics.GetActorOfClass` "/Game/Core/Cameras/BP_MainCamera.BP_MainCamera_C"))
      (`/Engine/EditorBlueprintResources/StandardMacros.IsValid` _returnvalue
        (:`Is Valid`
          (set `self.MainCamera` _returnvalue))
        (:`Is Not Valid`
          (bind _returnvalue_2 (`|SpawnActorFromClass` "/Game/Core/Cameras/BP_MainCamera.BP_MainCamera_C" (`KismetMathLibrary.MakeTransform` (0.0 0.0 0.0)) "Undefined" "MultiplyWithRoot" null null))
          (set `self.MainCamera` _returnvalue_2))))
    (:`then_1`
      (`self.SetViewTargetWithBlend` (`self.MainCamera`)))))

(fn `UserConstructionScript`)